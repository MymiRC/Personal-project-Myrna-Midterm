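; BP_Arrow is an arrow projectile that is launched at a given velocity and halts on its first overlap.
; Shoot sets the ProjectileMovement speeds, fires along local X, enables query-only collision on the Box and turns on mesh physics simulation.
; The Box overlap stops and deactivates the movement and disables Box collision, leaving the mesh's physics setting untouched.
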(event `Shoot`
  (params (Velocity :type "Float (double-precision)"))
  (bind _projectilemovement (`self.ProjectileMovement`))
  (bind _output_get (set `ProjectileMovementComponent.MaxSpeed` Velocity _projectilemovement))
  (set `ProjectileMovementComponent.InitialSpeed` _output_get _projectilemovement)
  (`ProjectileMovementComponent.SetVelocityInLocalSpace` _projectilemovement (`KismetMathLibrary.MakeVector` Velocity))
  (`ActorComponent.SetActive` (`self.ProjectileMovement`) true false)
  (`PrimitiveComponent.SetCollisionEnabled` (`self.Box`) "QueryOnly")
  (`PrimitiveComponent.SetSimulatePhysics` (`self.StaticMeshComponent`) true))

(event `self.Box.OnComponentBeginOverlap`
  (params (OverlappedComponent :type "PrimitiveComponent Object Reference") (OtherActor :type "Actor Object Reference") (OtherComp :type "PrimitiveComponent Object Reference") (OtherBodyIndex :type Integer) (bFromSweep :type Boolean) (SweepResult :type "HitResult Structure (by ref)"))
  (bind _projectilemovement (`self.ProjectileMovement`))
  (`MovementComponent.StopMovementImmediately` _projectilemovement)
  (`ActorComponent.SetActive` _projectilemovement false false)
  (`PrimitiveComponent.SetCollisionEnabled` (`self.Box`) "NoCollision"))

(fn `UserConstructionScript`)