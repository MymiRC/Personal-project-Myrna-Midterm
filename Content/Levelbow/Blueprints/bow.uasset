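; VR bow Actor held in one hand and drawn with the other, firing arrows when the string hand lets go.
; The first Pickup attaches the bow to the hand; a second, overlapping the string, spawns an arrow on it and enables Tick.
; Tick projects that hand onto the bow's axis to move the string and measure charge, drawing a debug sphere.
; Release plays a SnapBack timeline that launches the arrow with charge-scaled strength.
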(event `/Game/VirtualRealityBP/Blueprints/PickupActorInterface.Pickup`
  (params (MotionController :type "SceneComponent Object Reference") (HandMesh :type "SceneComponent Object Reference"))
  (`self.FirstHand`
    (:`then`
      (for _array_element (`PrimitiveComponent.GetOverlappingActors` (`self.stringcollision`) "/Script/Engine.Actor")
        (if (== _array_element (`ActorComponent.GetOwner` MotionController))
          (set `self.SecondHand` MotionController)
          (`self.SetActorTickEnabled` true)
          (bind _returnvalue (`|SpawnActorFromClass` "/Game/Levelbow/Blueprints/pickable_arrow.pickable_arrow_C" (`KismetMathLibrary.MakeTransform` (0.0 0.0 0.0)) "AlwaysSpawn" "OverrideRootScale" null null))
          (bind _output_get (set `self.aRROW` _returnvalue))
          (`self.K2_AttachToComponent` _output_get (`self.String`) "None" "SnapToTarget" "SnapToTarget" "KeepWorld" true))))
    (:`else`
      (bind _output_get_2 (set `self.FirstHand` HandMesh))
      (`SceneComponent.K2_AttachToComponent` (`self.StaticMeshComponent`) _output_get_2 "bow" "SnapToTarget" "SnapToTarget" "KeepWorld" false))))

(event `/Game/VirtualRealityBP/Blueprints/PickupActorInterface.Drop`
  (params (MotionController :type "SceneComponent Object Reference") (HandMesh :type "SceneComponent Object Reference"))
  (bind _secondhand (`self.SecondHand`)
    (:`then`
      (if (== _secondhand MotionController)
        (set `self.SecondHand` null)
        (`self.SetActorTickEnabled` false)
        (`self.Shoot`)))
    (:`else`
      (bind _firsthand (`self.FirstHand`)
        (:`then`
          (if (== _firsthand HandMesh)
            (`self.K2_DetachFromActor` "KeepWorld" "KeepWorld" "KeepWorld")
            (set `self.FirstHand` null)
            (set `self.SecondHand` null)))
        (:`else`)))))

(event `Shoot`
  (`TimelineComponent.SetPlayRate` (`self.SnapBack`) (/ 1.0 0.05))
  (bind (_direction _newtrack_1) (`Timeline|SnapBack` :!via `PlayFromStart`)
    (:`Update`
      (`SceneComponent.K2_SetRelativeLocation` (`self.String`) (`KismetMathLibrary.VLerp` (`self.StringRelativeLocation`) (`SceneComponent.RelativeLocation` (`self.stringcollision`)) _newtrack_1) false false)
      (if (> _newtrack_1 0.8)
        (bind _arrow (`self.aRROW`)
          (:`then`
            (`self.K2_DetachFromActor` _arrow "KeepWorld" "KeepWorld" "KeepWorld")
            (`/Game/Levelbow/Blueprints/pickable_arrow.Shoot` _arrow (`KismetMathLibrary.MapRangeClamped` (`self.SpringCharge`) 0.0 60.0 1000.0 3000.0)))
          (:`else`))))))

(event `self.ReceiveTick`
  (params (DeltaSeconds :type "Float (single-precision)"))
  (bind _returnvalue (- (`self.StringRelativeLocation`) (`SceneComponent.RelativeLocation` (`self.stringcollision`))))
  (bind _returnvalue_2 (`KismetMathLibrary.VSize` _returnvalue))
  (bind _secondhand (`self.SecondHand`)
    (:`then`
      (bind _returnvalue_3 (`KismetMathLibrary.ProjectVectorOnToVector` (`KismetMathLibrary.InverseTransformLocation` (`self.GetTransform`) (`SceneComponent.K2_GetComponentLocation` _secondhand)) (`KismetMathLibrary.Conv_RotatorToVector` (`SceneComponent.RelativeRotation` (`self.StaticMeshComponent`)))))
      (`KismetSystemLibrary.DrawDebugSphere` _returnvalue_3 5.0 6 (struct :`R` 1.0 :`G` 0.152145 :`B` 0.752857 :`A` 1.0) 0.1)
      (bind _output_get (set `self.StringRelativeLocation` _returnvalue_3))
      (set `self.SpringCharge` _returnvalue_2)
      (if (and (< (`KismetMathLibrary.Dot_VectorVector` (`KismetMathLibrary.Normal` _returnvalue) (`KismetMathLibrary.Conv_RotatorToVector` (`SceneComponent.RelativeRotation` (`self.StaticMeshComponent`)))) 0.0) (< _returnvalue_2 60.0))
        (`SceneComponent.K2_SetRelativeLocation` (`self.String`) _output_get false false)))
    (:`else`)))

(fn `UserConstructionScript`)