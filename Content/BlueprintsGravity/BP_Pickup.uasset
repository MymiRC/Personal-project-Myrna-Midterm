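; BP_Pickup is a static mesh actor that BP_MotionController can pick up, and that plays a sound and destroys itself on overlap.
; Physics stays off from BeginPlay, and Pickup attaches the root component to the given component, keeping world transform.
; Any mesh overlap triggers the sound at world origin, then destruction.
; Drop is empty, as its physics and detach nodes are left unconnected.
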(event `self.ReceiveBeginPlay`
  (`PrimitiveComponent.SetSimulatePhysics` (`self.StaticMeshComponent`) false))

(event `/Game/BlueprintsGravity/PickupActorInterface.Pickup`
  (params (AttachTo :type "SceneComponent Object Reference"))
  (`PrimitiveComponent.SetSimulatePhysics` (`self.StaticMeshComponent`) false)
  (`SceneComponent.K2_AttachToComponent` (`self.K2_GetRootComponent`) AttachTo "None" "KeepWorld" "KeepWorld" "KeepWorld" false))

(event `/Game/BlueprintsGravity/PickupActorInterface.Drop`)

(event `self.StaticMeshComponent.OnComponentBeginOverlap`
  (params (OverlappedComponent :type "PrimitiveComponent Object Reference") (OtherActor :type "Actor Object Reference") (OtherComp :type "PrimitiveComponent Object Reference") (OtherBodyIndex :type Integer) (bFromSweep :type Boolean) (SweepResult :type "HitResult Structure (by ref)"))
  (`GameplayStatics.PlaySoundAtLocation` "/Game/Levelbow/Audio/ding-idea-40142__1_.ding-idea-40142__1_" (0.0 0.0 0.0) (struct) 1.0 1.0 0.0 null null null)
  (`self.K2_DestroyActor`))

(fn `UserConstructionScript`)