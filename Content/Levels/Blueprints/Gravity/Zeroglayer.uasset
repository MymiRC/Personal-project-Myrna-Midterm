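; Zero-gravity VR player character that moves by grabbing gravity cubes with either motion controller and flinging itself off them.
; Grab inputs find a cube via a capsule overlap at the hand and store that hand and its grab point on the cube.
; While holding, Tick shifts the player opposite to hand movement.
; On release, a DoOnce sets launch velocity from the gap between the actor and its smoothed, trailing position.
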(event `self.ReceiveBeginPlay`
  (set `self.Current location` (`self.K2_GetActorLocation`)))

(event `self.ReceiveTick`
  (params (DeltaSeconds :type "Float (single-precision)"))
  (`KismetSystemLibrary.PrintString` (`KismetStringLibrary.Conv_VectorToString` (stale _output_get)))
  (set `self.Current location` (`KismetMathLibrary.VInterpTo` (`self.Current location`) (`self.K2_GetActorLocation`) DeltaSeconds 1.0))
  (bind _grabcube (`self.Grabcube`)
    (:`then`
      (`self.K2_SetActorLocation` (+ (`self.K2_GetActorLocation`) (- (`/Game/Levels/Blueprints/Gravity/gravitycube.grablocation` _grabcube) (`SceneComponent.K2_GetComponentLocation` (`/Game/Levels/Blueprints/Gravity/gravitycube.grabbinghands` _grabcube)))))
      (goto _label :!via `Reset`))
    (:`else`
      (`/Engine/EditorBlueprintResources/StandardMacros.DoOnce` true :!label _label
        (:`Completed`
          (bind _output_get (set `MovementComponent.Velocity` (* (- (`self.K2_GetActorLocation`) (`self.Current location`)) 5.0) (`self.CharacterMovement`))))))))

(event `InputAction|GrabLeft`
  (params (Key :type "Key Structure"))
  (bind _motioncontrollerleft (`self.MotionControllerleft`))
  ;[1 1 1] Grabbing gravity cube
  (:`Pressed`
    (bind _outactors (`KismetSystemLibrary.CapsuleOverlapActors` (`SceneComponent.K2_GetComponentLocation` (`self.MotionControllerleft`)) 20.0 20.0 (`|MakeArray` "ObjectTypeQuery2" :!type "EObjectTypeQuery Enum")))
    (for _array_element _outactors
      (bind _asgravitycube (cast `/Game/Levels/Blueprints/Gravity/gravitycube` _array_element))
      (bind _output_get (set `self.Grabcube` _asgravitycube))
      (set `/Game/Levels/Blueprints/Gravity/gravitycube.grabbinghands` _motioncontrollerleft _output_get)
      (set `/Game/Levels/Blueprints/Gravity/gravitycube.grablocation` (`SceneComponent.K2_GetComponentLocation` _motioncontrollerleft) _output_get)
      (break)))
  (:`Released`
    (bind _grabcube (`self.Grabcube`)
      (:`then`
        (set `/Game/Levels/Blueprints/Gravity/gravitycube.grabbinghands` null _grabcube)
        (set `self.Grabcube` null))
      (:`else`))))

(event `InputAction|GrabRight`
  (params (Key :type "Key Structure"))
  (bind _motioncontrollerright (`self.MotionControllerright`))
  ;[1 1 1] Grabbing gravity cube
  (:`Pressed`
    (bind _outactors (`KismetSystemLibrary.CapsuleOverlapActors` (`SceneComponent.K2_GetComponentLocation` (`self.MotionControllerright`)) 20.0 20.0 (`|MakeArray` "ObjectTypeQuery2" :!type "EObjectTypeQuery Enum")))
    (for _array_element _outactors
      (`self.SetActorHiddenInGame` _array_element false)
      (bind _asgravitycube (cast `/Game/Levels/Blueprints/Gravity/gravitycube` _array_element))
      (bind _output_get (set `self.Grabcube` _asgravitycube))
      (set `/Game/Levels/Blueprints/Gravity/gravitycube.grabbinghands` _motioncontrollerright _output_get)
      (set `/Game/Levels/Blueprints/Gravity/gravitycube.grablocation` (`SceneComponent.K2_GetComponentLocation` _motioncontrollerright) _output_get)
      (break)))
  (:`Released`
    (bind _grabcube (`self.Grabcube`)
      (:`then`
        (set `/Game/Levels/Blueprints/Gravity/gravitycube.grabbinghands` null _grabcube)
        (set `self.Grabcube` null))
      (:`else`))))

(fn `UserConstructionScript`)