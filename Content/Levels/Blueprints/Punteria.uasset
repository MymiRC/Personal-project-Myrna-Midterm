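; Punteria is an actor Blueprint that keeps score for what appears to be an aiming target with three scoring zones.
; Overlap events on components named 10, 25 and 50 each add the matching points to Score and print a colored bonus message.
; All three paths then share a debug print of the running total, prefixed with "Tocó".
; The overlap handlers do not filter which actor or component triggered them.
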(event `self.10.OnComponentBeginOverlap`
  (params (OverlappedComponent :type "PrimitiveComponent Object Reference") (OtherActor :type "Actor Object Reference") (OtherComp :type "PrimitiveComponent Object Reference") (OtherBodyIndex :type Integer) (bFromSweep :type Boolean) (SweepResult :type "HitResult Structure (by ref)"))
  (bind _score (`self.Score`))
  (set `self.Score` (+ _score 10))
  (`KismetSystemLibrary.PrintString` "+10" true true (struct :`R` 0.181164 :`G` 0.48515 :`B` 0.035601 :`A` 1.0))
  (`KismetSystemLibrary.PrintString` (`KismetStringLibrary.Concat_StrStr` "Tocó " (`KismetStringLibrary.Conv_IntToString` _score)) :!label _label))

(event `self.25.OnComponentBeginOverlap`
  (params (OverlappedComponent :type "PrimitiveComponent Object Reference") (OtherActor :type "Actor Object Reference") (OtherComp :type "PrimitiveComponent Object Reference") (OtherBodyIndex :type Integer) (bFromSweep :type Boolean) (SweepResult :type "HitResult Structure (by ref)"))
  (set `self.Score` (+ (`self.Score`) 25))
  (`KismetSystemLibrary.PrintString` "+25" true true (struct :`R` 1.0 :`G` 0.41479 :`A` 1.0))
  (goto _label))

(event `self.50.OnComponentBeginOverlap`
  (params (OverlappedComponent :type "PrimitiveComponent Object Reference") (OtherActor :type "Actor Object Reference") (OtherComp :type "PrimitiveComponent Object Reference") (OtherBodyIndex :type Integer) (bFromSweep :type Boolean) (SweepResult :type "HitResult Structure (by ref)"))
  (set `self.Score` (+ (`self.Score`) 50))
  (`KismetSystemLibrary.PrintString` "+50" true true (struct :`R` 1.0 :`G` 0.41479 :`A` 1.0))
  (goto _label))

(fn `UserConstructionScript`)