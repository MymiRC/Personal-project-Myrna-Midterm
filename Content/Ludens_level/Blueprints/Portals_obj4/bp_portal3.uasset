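; Portal 3 actor for the Ludens level, gating its logic on normal world-to-meters scale (100).
; Box overlaps fire the portal-overlapped dispatcher for actors not tagged hand or spaceship, and a character's first entry notifies the miniature portal that the third object is found.
; Box1 plays a sequence forward, reversed after exit delays, toggling Bp_portal4's Portalv42 visibility and the plane's portal/blue material when scale allows.
; Construction captures the Portalv4 scene.
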(event `self.Box.OnComponentBeginOverlap`
  (params (OverlappedComponent :type "PrimitiveComponent Object Reference") (OtherActor :type "Actor Object Reference") (OtherComp :type "PrimitiveComponent Object Reference") (OtherBodyIndex :type Integer) (bFromSweep :type Boolean) (SweepResult :type "HitResult Structure (by ref)"))
  (`|ExecutionSequence`
    (:`then_0`
      (if (and (== (`HeadMountedDisplayFunctionLibrary.GetWorldToMetersScale`) 100.0) (and (not (`self.ActorHasTag` OtherActor "hand")) (not (`self.ActorHasTag` OtherActor "spaceship"))))
        (`self.Portal1isoverlapped` (0.0 0.0 0.0) (0.0 0.0 0.0) OtherActor)))
    (:`then_1`
      (if (and (`self.ActorHasTag` OtherActor "character") (== (`HeadMountedDisplayFunctionLibrary.GetWorldToMetersScale`) 100.0))
        (`/Engine/EditorBlueprintResources/StandardMacros.DoOnce` false
          (:`Completed`
            (bind _outactors (`GameplayStatics.GetAllActorsOfClass` "/Game/portalminiature_Blueprint.portalminiature_Blueprint_C"))
            (`/Game/portalminiature_Blueprint.3rd object founded` (`|GetArrayItem` _outactors))))))))

(event `self.Box1.OnComponentBeginOverlap`
  (params (OverlappedComponent :type "PrimitiveComponent Object Reference") (OtherActor :type "Actor Object Reference") (OtherComp :type "PrimitiveComponent Object Reference") (OtherBodyIndex :type Integer) (bFromSweep :type Boolean) (SweepResult :type "HitResult Structure (by ref)"))
  (bind _sequenceplayer (`ActorSequenceComponent.SequencePlayer` (`self.Anim`)))
  (if (and (== (`HeadMountedDisplayFunctionLibrary.GetWorldToMetersScale`) 100.0) (not (`self.ActorHasTag` OtherActor "spaceship")))
    (bind _outactors (`GameplayStatics.GetAllActorsOfClass` "/Game/Ludens_level/Blueprints/Portals_obj4/bp_portal4.bp_portal4_C"))
    (bind _portalv42 (`/Game/Ludens_level/Blueprints/Portals_obj4/bp_portal4.portalv42` (`|GetArrayItem` _outactors)))
    (`/Engine/EditorBlueprintResources/StandardMacros.IsValid` _portalv42
      (:`Is Valid`
        (`SceneComponent.SetVisibility` _portalv42 true false)
        (`MovieSceneSequencePlayer.Play` _sequenceplayer)
        (`PrimitiveComponent.SetMaterial` (`self.Plane`) 0 "/Game/Ludens_level/Assets/portal/portalv42.portalv42")))
    (else
      (`MovieSceneSequencePlayer.Play` _sequenceplayer))))

(event `self.Box1.OnComponentEndOverlap`
  (params (OverlappedComponent :type "PrimitiveComponent Object Reference") (OtherActor :type "Actor Object Reference") (OtherComp :type "PrimitiveComponent Object Reference") (OtherBodyIndex :type Integer))
  (bind _sequenceplayer (`ActorSequenceComponent.SequencePlayer` (`self.Anim`)))
  (`KismetSystemLibrary.Delay` 1.0)
  (if (and (== (`HeadMountedDisplayFunctionLibrary.GetWorldToMetersScale`) 100.0) (not (`self.ActorHasTag` OtherActor "spaceship")))
    (`KismetSystemLibrary.Delay` 0.2)
    (bind _portalv42 (`/Game/Ludens_level/Blueprints/Portals_obj4/bp_portal4.portalv42` (`|GetArrayItem` (stale `self.Box1.OnComponentBeginOverlap` _outactors))))
    (`/Engine/EditorBlueprintResources/StandardMacros.IsValid` _portalv42
      (:`Is Valid`
        (`SceneComponent.SetVisibility` _portalv42 false false)
        (`MovieSceneSequencePlayer.PlayReverse` _sequenceplayer)
        (`PrimitiveComponent.SetMaterial` (`self.Plane`) 0 "/Game/StarterContent/Materials/blue.blue")))
    (else
      (`MovieSceneSequencePlayer.PlayReverse` _sequenceplayer))))

(fn `UserConstructionScript`
  (`SceneCaptureComponentCube.CaptureScene` (`self.portalv4`)))