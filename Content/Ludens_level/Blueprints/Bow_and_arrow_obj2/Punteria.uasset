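; Archery target that scores hits from arrow-tagged actors on its ring components, each worth its own points.
; Each hit briefly swaps that ring's material as feedback, then updates the high score; a separate event counts arrows.
; The first bullseye also fires a one-time reward: it opens the chest, moves the bow to a TargetPoint, starts it rotating and reveals a VR quote.
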(event `self.10.OnComponentBeginOverlap`
  (params (OverlappedComponent :type "PrimitiveComponent Object Reference") (OtherActor :type "Actor Object Reference") (OtherComp :type "PrimitiveComponent Object Reference") (OtherBodyIndex :type Integer) (bFromSweep :type Boolean) (SweepResult :type "HitResult Structure (by ref)"))
  (bind _10 (`self.10`))
  ;[1 1 1] Add points when overlapped part of the aim
  (if (`self.ActorHasTag` OtherActor "arrow")
    (set `self.Score` (+ (`self.Score`) 10))
    (`PrimitiveComponent.SetMaterial` _10 0 "/Game/VirtualReality/Materials/color.color")
    (`KismetSystemLibrary.Delay` 0.2)
    (`PrimitiveComponent.SetMaterial` _10 0 "/Game/StarterContent/Materials/blue.blue")
    (`self.highestscoreupdate` :!label _label)))

(event `self.25.OnComponentBeginOverlap`
  (params (OverlappedComponent :type "PrimitiveComponent Object Reference") (OtherActor :type "Actor Object Reference") (OtherComp :type "PrimitiveComponent Object Reference") (OtherBodyIndex :type Integer) (bFromSweep :type Boolean) (SweepResult :type "HitResult Structure (by ref)"))
  (bind _25 (`self.25`))
  ;[1 1 1] Add points when overlapped part of the aim
  (if (`self.ActorHasTag` OtherActor "arrow")
    (set `self.Score` (+ (`self.Score`) 25))
    (`PrimitiveComponent.SetMaterial` _25 0 "/Game/VirtualReality/Materials/color.color")
    (`KismetSystemLibrary.Delay` 0.2)
    (`PrimitiveComponent.SetMaterial` _25 0 "/Game/StarterContent/Materials/pink_Inst.pink_Inst")
    (goto _label)))

(event `self.50.OnComponentBeginOverlap`
  (params (OverlappedComponent :type "PrimitiveComponent Object Reference") (OtherActor :type "Actor Object Reference") (OtherComp :type "PrimitiveComponent Object Reference") (OtherBodyIndex :type Integer) (bFromSweep :type Boolean) (SweepResult :type "HitResult Structure (by ref)"))
  (bind _50 (`self.50`))
  ;[1 1 1] Add points when overlapped part of the aim
  (if (`self.ActorHasTag` OtherActor "arrow")
    (set `self.Score` (+ (`self.Score`) 50))
    (`PrimitiveComponent.SetMaterial` _50 0 "/Game/VirtualReality/Materials/color.color")
    (`|ExecutionSequence`
      (:`then_0`
        (`/Engine/EditorBlueprintResources/StandardMacros.DoOnce` false
          (:`Completed`
            (`self.after object 1`))))
      (:`then_1`
        (`KismetSystemLibrary.Delay` 0.5)
        (`PrimitiveComponent.SetMaterial` _50 0 "/Game/StarterContent/Materials/pink.pink")
        (goto _label)))))

(event `self.15.OnComponentBeginOverlap`
  (params (OverlappedComponent :type "PrimitiveComponent Object Reference") (OtherActor :type "Actor Object Reference") (OtherComp :type "PrimitiveComponent Object Reference") (OtherBodyIndex :type Integer) (bFromSweep :type Boolean) (SweepResult :type "HitResult Structure (by ref)"))
  (bind _15 (`self.15`))
  ;[1 1 1] Add points when overlapped part of the aim
  (if (`self.ActorHasTag` OtherActor "arrow")
    (set `self.Score` (+ (`self.Score`) 15))
    (`PrimitiveComponent.SetMaterial` _15 0 "/Game/VirtualReality/Materials/color.color")
    (`KismetSystemLibrary.Delay` 0.5)
    (`PrimitiveComponent.SetMaterial` _15 0 "/Game/Ludens_level/Assets/MAterial_fade/lambert1.lambert1")
    (goto _label)))

(event `Sum arrow`
  (set `self.arrows` (+ (`self.arrows`) 1)))

(event `after object 1`
  (bind _outactors (`GameplayStatics.GetAllActorsOfClass` "/Game/Ludens_level/Assets/Meshes_final_version/chest2_Blueprint.chest2_Blueprint_C"))
  (`/Game/Ludens_level/Assets/Meshes_final_version/chest2_Blueprint.ChestOpens` (`|GetArrayItem` _outactors))
  (`KismetSystemLibrary.Delay` 2.0)
  (bind _outactors_2 (`GameplayStatics.GetAllActorsOfClass` "/Game/Ludens_level/Assets/Bow_and_arrow/bow_mesh_v3_Blueprint.bow_mesh_v3_Blueprint_C"))
  (bind _outactors_3 (`GameplayStatics.GetAllActorsOfClass` "/Script/Engine.TargetPoint"))
  (bind _output (`|GetArrayItem` _outactors_2))
  (`self.K2_SetActorLocation` _output (`self.K2_GetActorLocation` (`|GetArrayItem` _outactors_3 2)) false false)
  (set `/Game/Ludens_level/Assets/Bow_and_arrow/bow_mesh_v3_Blueprint.rotate` true _output)
  (bind _outactors_4 (`GameplayStatics.GetAllActorsOfClass` "/Game/Ludens_level/Blueprints/Widgets/quote1vr.quote1vr_C"))
  (`/Game/Ludens_level/Blueprints/Widgets/quote1vr.Appear phrase` (`|GetArrayItem` _outactors_4)))

(fn `highestscoreupdate`
  (bind _score (`self.Score`))
  (if (> _score (`self.highscore`))
    (set `self.highscore` _score)))

(fn `UserConstructionScript`)