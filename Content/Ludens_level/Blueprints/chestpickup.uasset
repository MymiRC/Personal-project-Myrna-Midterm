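; A VR chest actor that can be picked up by motion controllers and toggles open or closed when touched by a hand.
; Pickup disables physics and attaches the mesh to the hand, while Drop detaches it and restores physics.
; Sphere overlap with "hand"-tagged actors alternates open and close through a FlipFlop, gated by a DoOnce with a delayed reset.
; Each state plays a level sequence and snaps a mesh's pitch.
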(event `/Game/VirtualRealityBP/Blueprints/PickupActorInterface2.Pickup`
  (params (MotionController :type "SceneComponent Object Reference") (HandMesh :type "SceneComponent Object Reference"))
  (bind _staticmeshcomponent (`self.StaticMeshComponent`))
  (`PrimitiveComponent.SetSimulatePhysics` _staticmeshcomponent false)
  (`SceneComponent.K2_AttachToComponent` _staticmeshcomponent HandMesh "None" "KeepWorld" "KeepWorld" "KeepWorld" false))

(event `/Game/VirtualRealityBP/Blueprints/PickupActorInterface2.Drop`
  (params (MotionController :type "SceneComponent Object Reference") (HandMesh :type "SceneComponent Object Reference"))
  (`PrimitiveComponent.SetSimulatePhysics` (`self.StaticMeshComponent`) true)
  (`self.K2_DetachFromActor` "KeepWorld" "KeepWorld" "KeepWorld"))

(event `ChestOpens`
  (bind _staticmesh (`self.StaticMesh`))
  (bind (_returnvalue_roll _returnvalue_pitch _returnvalue_yaw) (`KismetMathLibrary.BreakRotator` (`SceneComponent.GetSocketRotation` _staticmesh "None")))
  (bind _sequenceplayer (`ActorSequenceComponent.SequencePlayer` (`self.chestfinal`)))
  (`MovieSceneSequencePlayer.Play` _sequenceplayer)
  (`SceneComponent.K2_SetRelativeRotation` _staticmesh (`KismetMathLibrary.MakeRotator` _returnvalue_roll -113.75499 _returnvalue_yaw) false false)
  (`MovieSceneSequencePlayer.Play` _sequenceplayer))

(event `ChestCloses`
  (bind _staticmesh (`self.StaticMesh`))
  (bind (_returnvalue_roll _returnvalue_pitch _returnvalue_yaw) (`KismetMathLibrary.BreakRotator` (`SceneComponent.GetSocketRotation` _staticmesh "None")))
  (bind _sequenceplayer (`ActorSequenceComponent.SequencePlayer` (`self.chestfinal1`)))
  (`MovieSceneSequencePlayer.Play` _sequenceplayer)
  (`SceneComponent.K2_SetRelativeRotation` _staticmesh (`KismetMathLibrary.MakeRotator` _returnvalue_roll 1.277 _returnvalue_yaw) false false)
  (`MovieSceneSequencePlayer.Play` _sequenceplayer))

(event `self.Sphere.OnComponentBeginOverlap`
  (params (OverlappedComponent :type "PrimitiveComponent Object Reference") (OtherActor :type "Actor Object Reference") (OtherComp :type "PrimitiveComponent Object Reference") (OtherBodyIndex :type Integer) (bFromSweep :type Boolean) (SweepResult :type "HitResult Structure (by ref)"))
  (if (`self.ActorHasTag` OtherActor "hand")
    (`/Engine/EditorBlueprintResources/StandardMacros.DoOnce` false :!label _label
      (:`Completed`
        (`/Engine/EditorBlueprintResources/StandardMacros.FlipFlop`
          (:`A`
            (`self.ChestOpens`)
            (`KismetSystemLibrary.Delay` 1.0)
            (goto _label :!via `Reset`))
          (:`B`
            (`self.ChestCloses`)
            (`KismetSystemLibrary.Delay` 1.0)
            (goto _label :!via `Reset`)))))))

(fn `UserConstructionScript`)