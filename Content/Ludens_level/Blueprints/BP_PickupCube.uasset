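; BP_PickupCube is a VR cube that reacts to being touched by the MotionControllerPawn's controllers.
; When a controller stops overlapping its mesh, it responds only if world-to-meters scale is default (100) and the pawn is stationary.
; It rumbles that controller, briefly disables overlap events as a debounce, then calls Touchedbybigcube and temporarily swaps its material to flash a color.
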(event `self.StaticMeshComponent.OnComponentEndOverlap`
  (params (OverlappedComponent :type "PrimitiveComponent Object Reference") (OtherActor :type "Actor Object Reference") (OtherComp :type "PrimitiveComponent Object Reference") (OtherBodyIndex :type Integer))
  (bind _staticmeshcomponent (`self.StaticMeshComponent`))
  ;[1 1 1] Call event when a static mesh ends overlapp
  (if (== (`HeadMountedDisplayFunctionLibrary.GetWorldToMetersScale`) 100.0)
    (bind _outactors (`GameplayStatics.GetAllActorsOfClass` "/Game/VirtualRealityBP/Blueprints/MotionControllerPawn.MotionControllerPawn_C"))
    (bind _output (`|GetArrayItem` _outactors))
    (if (and (or (== OtherActor (`/Game/VirtualRealityBP/Blueprints/MotionControllerPawn.LeftController` _output)) (== (`/Game/VirtualRealityBP/Blueprints/MotionControllerPawn.RightController` _output) OtherActor)) (== (`self.GetVelocity` _output) (0.0 0.0 0.0)))
      (`self.Haptics` OtherActor)
      (set `PrimitiveComponent.bGenerateOverlapEvents` false (`self.StaticMeshComponent`))
      (`KismetSystemLibrary.Delay` 0.3)
      (set `PrimitiveComponent.bGenerateOverlapEvents` true (`self.StaticMeshComponent`))
      (`PrimitiveComponent.SetMaterial` _staticmeshcomponent 0 "/Game/VirtualReality/Materials/color.color")
      (`self.Touchedbybigcube`)
      (`KismetSystemLibrary.Delay` 1.0)
      (`PrimitiveComponent.SetMaterial` _staticmeshcomponent 0 "/Game/Ludens_level/Audio/blinn1.blinn1"))))

(fn `Haptics`
  (params (B :type "Object Object Reference"))
  (bind _outactors (`GameplayStatics.GetAllActorsOfClass` "/Game/VirtualRealityBP/Blueprints/MotionControllerPawn.MotionControllerPawn_C"))
  (bind _output (`|GetArrayItem` _outactors))
  (bind _leftcontroller (`/Game/VirtualRealityBP/Blueprints/MotionControllerPawn.LeftController` _output))
  (if (== B _leftcontroller)
    (`/Game/VirtualRealityBP/Blueprints/BP_MotionController1.RumbleController` _leftcontroller 1.0)
    (else
      (`/Game/VirtualRealityBP/Blueprints/BP_MotionController1.RumbleController` (`/Game/VirtualRealityBP/Blueprints/MotionControllerPawn.RightController` _output) 1.0))))

(fn `UserConstructionScript`)