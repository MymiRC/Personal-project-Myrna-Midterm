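; VR grabbable cube that BP_MotionController picks up by attaching its static mesh to the hand mesh, with Drop detaching it in place.
; Materialblinking loops through delays, alternating the M_ArcEndpoint highlight with the cube's own material while the Colorchange flag is set.
; Pickup or any overlap on the mesh clears Colorchange, so the blink loop ends back on the cube material.
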(event `/Game/VirtualRealityBP/Blueprints/PickupActorInterface2.Pickup`
  (params (MotionController :type "SceneComponent Object Reference") (HandMesh :type "SceneComponent Object Reference"))
  (set `self.colorchange` false)
  (`SceneComponent.K2_AttachToComponent` (`self.StaticMeshComponent`) HandMesh "None" "KeepWorld" "KeepWorld" "KeepWorld" false))

(event `/Game/VirtualRealityBP/Blueprints/PickupActorInterface2.Drop`
  (params (MotionController :type "SceneComponent Object Reference") (HandMesh :type "SceneComponent Object Reference"))
  (`self.K2_DetachFromActor` "KeepWorld" "KeepWorld" "KeepWorld"))

(event `Material blinking`
  (if (`self.colorchange`) :!label _label
    (`PrimitiveComponent.SetMaterial` (`self.StaticMeshComponent`) 0 "/Game/VirtualReality/Materials/M_ArcEndpoint.M_ArcEndpoint")
    (`KismetSystemLibrary.Delay` 1.0)
    (`PrimitiveComponent.SetMaterial` (`self.StaticMeshComponent`) 0 "/Game/Ludens_level/Blueprints/Geometry/Meshes/CubeMaterial.CubeMaterial")
    (`KismetSystemLibrary.Delay` 0.5)
    (goto _label)))

(event `self.StaticMeshComponent.OnComponentBeginOverlap`
  (params (OverlappedComponent :type "PrimitiveComponent Object Reference") (OtherActor :type "Actor Object Reference") (OtherComp :type "PrimitiveComponent Object Reference") (OtherBodyIndex :type Integer) (bFromSweep :type Boolean) (SweepResult :type "HitResult Structure (by ref)"))
  (set `self.colorchange` false))

(fn `UserConstructionScript`)