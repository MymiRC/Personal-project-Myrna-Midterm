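; VR eraser button that resets the score on the whiteboard.
; Any overlap on Box calls Ereaserfunc on the first BP_Whiteboard found in the level.
; A "hand"-tagged actor overlapping Box1 plays the ActorSequence and rumbles the matching MotionControllerPawn controller.
; A separate Haptics Effect function offers a stronger rumble but is not called in this graph.
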(event `self.Box.OnComponentBeginOverlap`
  (params (OverlappedComponent :type "PrimitiveComponent Object Reference") (OtherActor :type "Actor Object Reference") (OtherComp :type "PrimitiveComponent Object Reference") (OtherBodyIndex :type Integer) (bFromSweep :type Boolean) (SweepResult :type "HitResult Structure (by ref)"))
  ;[1 1 1] When collliding with object, score is reset
  (`|ExecutionSequence`
    (:`then_0`
      (bind _outactors (`GameplayStatics.GetAllActorsOfClass` "/Game/Ludens_level/Blueprints/Painting/BP_Whiteboard.BP_Whiteboard_C"))
      (`/Game/Ludens_level/Blueprints/Painting/BP_Whiteboard.Ereaserfunc` (`|GetArrayItem` _outactors)))))

(event `self.Box1.OnComponentBeginOverlap`
  (params (OverlappedComponent :type "PrimitiveComponent Object Reference") (OtherActor :type "Actor Object Reference") (OtherComp :type "PrimitiveComponent Object Reference") (OtherBodyIndex :type Integer) (bFromSweep :type Boolean) (SweepResult :type "HitResult Structure (by ref)"))
  (if (`self.ActorHasTag` OtherActor "hand")
    (`MovieSceneSequencePlayer.Play` (`ActorSequenceComponent.SequencePlayer` (`self.ActorSequence`)))
    (bind _outactors (`GameplayStatics.GetAllActorsOfClass` "/Game/VirtualRealityBP/Blueprints/MotionControllerPawn.MotionControllerPawn_C"))
    (bind _output (`|GetArrayItem` _outactors))
    (bind _leftcontroller (`/Game/VirtualRealityBP/Blueprints/MotionControllerPawn.LeftController` _output))
    (if (== OtherActor _leftcontroller)
      (`/Game/VirtualRealityBP/Blueprints/BP_MotionController1.RumbleController` _leftcontroller 1.0)
      (else
        (`/Game/VirtualRealityBP/Blueprints/BP_MotionController1.RumbleController` (`/Game/VirtualRealityBP/Blueprints/MotionControllerPawn.RightController` _output) 1.0)))))

(fn `Haptics Effect`
  (params (A :type "Object Object Reference"))
  (bind _outactors (`GameplayStatics.GetAllActorsOfClass` "/Game/VirtualRealityBP/Blueprints/MotionControllerPawn.MotionControllerPawn_C"))
  (bind _output (`|GetArrayItem` _outactors))
  (bind _leftcontroller (`/Game/VirtualRealityBP/Blueprints/MotionControllerPawn.LeftController` _output))
  (if (== A _leftcontroller)
    (`/Game/VirtualRealityBP/Blueprints/BP_MotionController1.RumbleController` _leftcontroller 1.5)
    (else
      (`/Game/VirtualRealityBP/Blueprints/BP_MotionController1.RumbleController` (`/Game/VirtualRealityBP/Blueprints/MotionControllerPawn.RightController` _output) 1.5))))

(fn `UserConstructionScript`)