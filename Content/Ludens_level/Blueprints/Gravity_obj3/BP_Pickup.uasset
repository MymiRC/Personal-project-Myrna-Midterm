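; BP_Pickup is a grabbable collectable that BP_MotionController picks up and that scores when it touches a "spaceship" tagged actor.
; Pickup attaches it with physics off, while Drop detaches it and enables physics.
; Spaceship overlap plays a sound and increments Rocket2collectable_Blueprint's Score.
; At the threshold it calls Call6ObjectsCollected, triggers 6thObjectFounded and Quote1vr_2's AppearPhrase once, then destroys itself.
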(event `self.ReceiveBeginPlay`
  (`PrimitiveComponent.SetSimulatePhysics` (`self.StaticMeshComponent`) false))

(event `/Game/Ludens_level/Blueprints/Gravity_obj3/PickupActorInterface.Pickup`
  (params (AttachTo :type "SceneComponent Object Reference"))
  (`PrimitiveComponent.SetSimulatePhysics` (`self.StaticMeshComponent`) false)
  (`SceneComponent.K2_AttachToComponent` (`self.K2_GetRootComponent`) AttachTo "None" "KeepWorld" "KeepWorld" "KeepWorld" false))

(event `/Game/Ludens_level/Blueprints/Gravity_obj3/PickupActorInterface.Drop`
  (`PrimitiveComponent.SetSimulatePhysics` (`self.StaticMeshComponent`) true)
  (`self.K2_DetachFromActor` "KeepWorld" "KeepWorld" "KeepWorld"))

(event `self.StaticMeshComponent.OnComponentBeginOverlap`
  (params (OverlappedComponent :type "PrimitiveComponent Object Reference") (OtherActor :type "Actor Object Reference") (OtherComp :type "PrimitiveComponent Object Reference") (OtherBodyIndex :type Integer) (bFromSweep :type Boolean) (SweepResult :type "HitResult Structure (by ref)"))
  (if (`self.ActorHasTag` OtherActor "spaceship")
    (`GameplayStatics.PlaySoundAtLocation` "/Game/Ludens_level/Audio/ding-idea-40142__1_.ding-idea-40142__1_" (0.0 0.0 0.0) (struct) 1.0 1.0 0.0 null null null)
    (bind _outactors (`GameplayStatics.GetAllActorsOfClass` "/Game/rocket2collectable_Blueprint.rocket2collectable_Blueprint_C"))
    (bind _output (`|GetArrayItem` _outactors))
    (bind _score (`/Game/rocket2collectable_Blueprint.score` _output))
    (set `/Game/rocket2collectable_Blueprint.score` (+ _score 1) _output)
    (if (>= _score 1)
      (`self.6 objects collected`)
      (`/Engine/EditorBlueprintResources/StandardMacros.DoOnce` false
        (:`Completed`
          (bind _outactors_2 (`GameplayStatics.GetAllActorsOfClass` "/Game/rocket2collectable_Blueprint.rocket2collectable_Blueprint_C"))
          (`/Game/rocket2collectable_Blueprint.6th object founded` (`|GetArrayItem` _outactors_2))
          (bind _outactors_3 (`GameplayStatics.GetAllActorsOfClass` "/Game/Ludens_level/Blueprints/Widgets/quote1vr_2.quote1vr_2_C"))
          (`/Game/Ludens_level/Blueprints/Widgets/quote1vr_2.Appear phrase` (`|GetArrayItem` _outactors_3))
          (`self.K2_DestroyActor`)))
      (else
        (`self.K2_DestroyActor`)))))

(fn `UserConstructionScript`)