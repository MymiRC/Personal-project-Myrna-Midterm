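; A VR pickup actor, gravityball1, that motion controllers can grab and release, with its static mesh held out of physics simulation from BeginPlay.
; Pickup disables physics, attaches the root to the given component keeping world transform, then calls HapticsEffect, while Drop enables physics and detaches.
; HapticsEffect requires the ball's "hand" tag and rumbles the first MotionControllerPawn's left controller if it matches the attach component, otherwise the right.
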(event `self.ReceiveBeginPlay`
  (`PrimitiveComponent.SetSimulatePhysics` (`self.StaticMeshComponent`) false))

(event `/Game/Ludens_level/Blueprints/Gravity_obj3/PickupActorInterface.Pickup`
  (params (AttachTo :type "SceneComponent Object Reference"))
  (`PrimitiveComponent.SetSimulatePhysics` (`self.StaticMeshComponent`) false)
  (`SceneComponent.K2_AttachToComponent` (`self.K2_GetRootComponent`) AttachTo "None" "KeepWorld" "KeepWorld" "KeepWorld" false)
  (`self.Haptics Effect` AttachTo))

(event `/Game/Ludens_level/Blueprints/Gravity_obj3/PickupActorInterface.Drop`
  (`PrimitiveComponent.SetSimulatePhysics` (`self.StaticMeshComponent`) true)
  (`self.K2_DetachFromActor` "KeepWorld" "KeepWorld" "KeepWorld"))

(fn `Haptics Effect`
  (params (A :type "Object Object Reference"))
  (if (`self.ActorHasTag` "hand")
    (bind _outactors (`GameplayStatics.GetAllActorsOfClass` "/Game/VirtualRealityBP/Blueprints/MotionControllerPawn.MotionControllerPawn_C"))
    (bind _output (`|GetArrayItem` _outactors))
    (bind _leftcontroller (`/Game/VirtualRealityBP/Blueprints/MotionControllerPawn.LeftController` _output))
    (if (== A _leftcontroller)
      (`/Game/VirtualRealityBP/Blueprints/BP_MotionController1.RumbleController` _leftcontroller 5.0)
      (else
        (`/Game/VirtualRealityBP/Blueprints/BP_MotionController1.RumbleController` (`/Game/VirtualRealityBP/Blueprints/MotionControllerPawn.RightController` _output) 5.0)))))

(fn `UserConstructionScript`)