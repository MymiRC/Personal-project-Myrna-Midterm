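; Costume5 is a VR costume pickup that the player puts on by touching it with a hand.
; Overlapping its box with a "hand"-tagged actor rumbles the matching controller and copies the costume mesh onto the MotionControllerPawn's Costumes component.
; The costume briefly swaps material as touch feedback, then a DoOnce tells Mirror3collectable_Blueprint that the fifth object is found.
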(event `self.BOXCollision.OnComponentBeginOverlap`
  (params (OverlappedComponent :type "PrimitiveComponent Object Reference") (OtherActor :type "Actor Object Reference") (OtherComp :type "PrimitiveComponent Object Reference") (OtherBodyIndex :type Integer) (bFromSweep :type Boolean) (SweepResult :type "HitResult Structure (by ref)"))
  (bind _costume (`self.costume`))
  (if (`self.ActorHasTag` OtherActor "hand")
    (`self.Haptics` OtherActor)
    (bind _outactors (`GameplayStatics.GetAllActorsOfClass` "/Game/VirtualRealityBP/Blueprints/MotionControllerPawn.MotionControllerPawn_C"))
    (bind _costumes (`/Game/VirtualRealityBP/Blueprints/MotionControllerPawn.Costumes` (`|GetArrayItem` _outactors)))
    (`StaticMeshComponent.SetStaticMesh` _costumes (`StaticMeshComponent.StaticMesh` (`self.costume`)))
    (`SceneComponent.SetWorldScale3D` _costumes (1.0 1.0 1.0))
    (`PrimitiveComponent.SetMaterial` _costume 0 "/Game/VirtualReality/Materials/M_ArcEndpoint.M_ArcEndpoint")
    (`KismetSystemLibrary.Delay` 1.0)
    (`PrimitiveComponent.SetMaterial` _costume 0 "/Game/Ludens_level/Assets/Meshes_final_version/_FRONT_427414._FRONT_427414")
    (`/Engine/EditorBlueprintResources/StandardMacros.DoOnce` false
      (:`Completed`
        (bind _outactors_2 (`GameplayStatics.GetAllActorsOfClass` "/Game/mirror3collectable_Blueprint.mirror3collectable_Blueprint_C"))
        (`/Game/mirror3collectable_Blueprint.5th object founded` (`|GetArrayItem` _outactors_2))))))

(fn `Haptics`
  (params (B :type "Object Object Reference"))
  (bind _outactors (`GameplayStatics.GetAllActorsOfClass` "/Game/VirtualRealityBP/Blueprints/MotionControllerPawn.MotionControllerPawn_C"))
  (bind _output (`|GetArrayItem` _outactors))
  (bind _leftcontroller (`/Game/VirtualRealityBP/Blueprints/MotionControllerPawn.LeftController` _output))
  (if (== _leftcontroller B)
    (`/Game/VirtualRealityBP/Blueprints/BP_MotionController1.RumbleController` _leftcontroller 0.5)
    (else
      (bind _rightcontroller (`/Game/VirtualRealityBP/Blueprints/MotionControllerPawn.RightController` _output))
      (if (== _rightcontroller B)
        (`/Game/VirtualRealityBP/Blueprints/BP_MotionController1.RumbleController` _rightcontroller 0.5)))))

(fn `UserConstructionScript`)