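; Whiteboard actor that a paint brush can draw on at runtime using a render target.
; On BeginPlay it creates the render target, feeds it to the mesh's canvas material as the brush stroke texture, and creates a dynamic brush material.
; OnPaintVisualTraceLine converts a hit to UVs with FindCollisionUV, passes position and the brush's size, color and strength to that material, then draws it into the render target.
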(event `self.ReceiveBeginPlay`
  (bind _returnvalue (`PrimitiveComponent.CreateDynamicMaterialInstance` (`self.StaticMeshComponent`) 0 "/Game/Ludens_level/Blueprints/Painting/M_BasicCanvas.M_BasicCanvas" "None"))
  (bind _returnvalue_2 (`KismetRenderingLibrary.CreateRenderTarget2D` (`self.RenderTextureSizeX`) (`self.RenderTextureSizeY`)))
  (set `self.RenderToTexture` _returnvalue_2)
  (`MaterialInstanceDynamic.SetTextureParameterValue` _returnvalue "BrushStroke" _returnvalue_2)
  (bind _returnvalue_3 (`KismetMaterialLibrary.CreateDynamicMaterialInstance` "/Game/Ludens_level/Blueprints/Painting/MI_PaintBrush_Inst.MI_PaintBrush_Inst"))
  (set `self.BrushMaterialInstance` _returnvalue_3))

(fn `OnPaintVisualTraceLine`
  (params (PaintBrush :type "/Game/Ludens_level/Blueprints/Painting/pencil Object Reference") (HitResult :type "HitResult Structure"))
  (bind (_x _y) (`KismetMathLibrary.BreakVector2D` (`GameplayStatics.FindCollisionUV` HitResult)))
  (set `self.Paint Brush` PaintBrush)
  (`MaterialInstanceDynamic.SetVectorParameterValue` (`self.BrushMaterialInstance`) "HitPosition" (make `LinearColor` _x _y 0.0 1.0))
  (`MaterialInstanceDynamic.SetScalarParameterValue` (`self.BrushMaterialInstance`) "BrushSize" (`/Game/Ludens_level/Blueprints/Painting/pencil.BrushSize` (`self.Paint Brush`)))
  (`MaterialInstanceDynamic.SetVectorParameterValue` (`self.BrushMaterialInstance`) "BrushColor" (`/Game/Ludens_level/Blueprints/Painting/pencil.BrushColor` (`self.Paint Brush`)))
  (`MaterialInstanceDynamic.SetScalarParameterValue` (`self.BrushMaterialInstance`) "BrushStrength" (`/Game/Ludens_level/Blueprints/Painting/pencil.BrushStrength` (`self.Paint Brush`)))
  (`KismetRenderingLibrary.DrawMaterialToRenderTarget` (`self.RenderToTexture`) (`self.BrushMaterialInstance`)))

(fn `UserConstructionScript`)