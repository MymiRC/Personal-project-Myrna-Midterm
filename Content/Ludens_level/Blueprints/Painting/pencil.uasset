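; VR pencil that can be picked up with a motion controller and used to paint on Whiteboard actors.
; Pickup turns off physics and attaches the mesh to the hand; Drop restores physics and detaches it.
; Every tick, a short complex line trace from the forward arrow looks for a Whiteboard, passing it the pencil as brush and the hit result to paint.
; Debug trace drawing and a print on each hit are left enabled.
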(event `self.ReceiveTick`
  (params (DeltaSeconds :type "Float (single-precision)"))
  (`parent.ReceiveTick` DeltaSeconds)
  (`self.Detect Hit Canvas Actor`))

(event `/Game/VirtualRealityBP/Blueprints/PickupActorInterface2.Pickup`
  (params (MotionController :type "SceneComponent Object Reference") (HandMesh :type "SceneComponent Object Reference"))
  (bind _staticmeshcomponent (`self.StaticMeshComponent`))
  (`PrimitiveComponent.SetSimulatePhysics` _staticmeshcomponent false)
  (`SceneComponent.K2_AttachToComponent` _staticmeshcomponent HandMesh "None" "KeepWorld" "KeepWorld" "KeepWorld" false))

(event `/Game/VirtualRealityBP/Blueprints/PickupActorInterface2.Drop`
  (params (MotionController :type "SceneComponent Object Reference") (HandMesh :type "SceneComponent Object Reference"))
  (`PrimitiveComponent.SetSimulatePhysics` (`self.StaticMeshComponent`) true)
  (`self.K2_DetachFromActor` "KeepWorld" "KeepWorld" "KeepWorld"))

(fn `Detect Hit Canvas Actor`
  (bind _arrowforward (`self.ArrowForward`))
  (bind _returnvalue (`SceneComponent.K2_GetComponentLocation` _arrowforward))
  (bind (_outhit _returnvalue_2) (`KismetSystemLibrary.LineTraceSingleByProfile` :`Start` _returnvalue :`End` (+ _returnvalue (* (`KismetMathLibrary.GetForwardVector` (`SceneComponent.K2_GetComponentRotation` _arrowforward)) 15.0)) :`ProfileName` "BlockAllDynamic" :`bTraceComplex` true :`DrawDebugType` "ForDuration"))
  (if _returnvalue_2
    (bind _aswhiteboard (cast `/Game/Ludens_level/Blueprints/Painting/Whiteboard` (`.HitActor` (`GameplayStatics.BreakHitResult` _outhit))))
    (`KismetSystemLibrary.PrintString` "Hello" true true (struct :`R` 1.0 :`G` 0.401133 :`B` 0.273084 :`A` 1.0))
    (`/Game/Ludens_level/Blueprints/Painting/Whiteboard.OnPaintVisualTraceLine` _aswhiteboard self _outhit)))

(fn `UserConstructionScript`)