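; Whiteboard Blueprint that players or other actors draw on by painting marker strokes into a render target.
; On BeginPlay, an eraser function creates a dynamic instance of the marker material and clears the render target to black.
; The DrawOnWhiteboard event passes a 2D location into that material and draws it to the render target, stamping a mark there.
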(event `self.ReceiveBeginPlay`
  (`self.Ereaserfunc`))

(event `DrawOnWhiteboard`
  (params (LocationToDraw :type "Vector2D Structure"))
  (bind _whiteboardmarker_mi (`self.WhiteboardMarker_MI`))
  (`MaterialInstanceDynamic.SetVectorParameterValue` _whiteboardmarker_mi "DrawLocationv1" (`KismetMathLibrary.Conv_VectorToLinearColor` (`KismetMathLibrary.Conv_Vector2DToVector` LocationToDraw)))
  (`KismetRenderingLibrary.DrawMaterialToRenderTarget` "/Game/Ludens_level/Blueprints/Painting/RT_Whiteboard.RT_Whiteboard" _whiteboardmarker_mi))

(fn `Ereaserfunc`
  (bind _returnvalue (`KismetMaterialLibrary.CreateDynamicMaterialInstance` "/Game/Ludens_level/Blueprints/Painting/M_WhiteboardMarker.M_WhiteboardMarker"))
  (set `self.WhiteboardMarker_MI` _returnvalue)
  (`KismetRenderingLibrary.ClearRenderTarget2D` "/Game/Ludens_level/Blueprints/Painting/RT_Whiteboard.RT_Whiteboard"))

(fn `UserConstructionScript`)