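; VR pencil that attaches to the hand on pickup and paints on a BP_Whiteboard.
; While an overlap flags painting, Tick line-traces briefly from the tip arrow and passes the hit's collision UV to the whiteboard, rumbling the controller.
; First pickup spawns the whiteboard and an eraser at a TargetPoint.
; First stroke notifies the pencil collectable and reveals a quote phrase.
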(event `self.ReceiveActorBeginOverlap`
  (params (OtherActor :type "Actor Object Reference"))
  (bind _staticmeshcomponent (`self.StaticMeshComponent`))
  (if (== (`self.Other Actor`) null)
    (set `self.Other Actor` OtherActor)
    (set `self.ispainting` true)
    (if (== (`HeadMountedDisplayFunctionLibrary.GetWorldToMetersScale`) 100.0)
      (`self.HapticsEffect` OtherActor)
      (`PrimitiveComponent.SetMaterial` _staticmeshcomponent 0 "/Game/VirtualReality/Materials/color.color")
      (`KismetSystemLibrary.Delay` 1.0)
      (`PrimitiveComponent.SetMaterial` _staticmeshcomponent 0 "/Game/StarterContent/Materials/blue.blue"))))

(event `self.ReceiveTick`
  (params (DeltaSeconds :type "Float (single-precision)"))
  (bind _arrowforward (`self.ArrowForward`))
  (bind _returnvalue (`SceneComponent.K2_GetComponentLocation` _arrowforward))
  (if (`self.ispainting`)
    (bind (_outhit _returnvalue_2) (`KismetSystemLibrary.LineTraceSingle` _returnvalue (+ _returnvalue (* (`KismetMathLibrary.GetForwardVector` (`SceneComponent.K2_GetComponentRotation` _arrowforward)) 15.0)) "TraceTypeQuery2"))
    (if _returnvalue_2
      (bind _asbp_whiteboard (cast `/Game/Ludens_level/Blueprints/Painting/BP_Whiteboard` (`.HitActor` (`GameplayStatics.BreakHitResult` _outhit))))
      (`/Game/Ludens_level/Blueprints/Painting/BP_Whiteboard.DrawOnWhiteboard` _asbp_whiteboard (`GameplayStatics.FindCollisionUV` _outhit))
      (`self.HapticsEffect` (`self.Other Actor`))
      (`/Engine/EditorBlueprintResources/StandardMacros.DoOnce` false
        (:`Completed`
          (bind _outactors (`GameplayStatics.GetAllActorsOfClass` "/Game/pencilcollectable_Blueprint.pencilcollectable_Blueprint_C"))
          (`/Game/pencilcollectable_Blueprint.2ndobjectfounded` (`|GetArrayItem` _outactors))
          (bind _outactors_2 (`GameplayStatics.GetAllActorsOfClass` "/Game/Ludens_level/Blueprints/Widgets/quote1vr_7.quote1vr_7_C"))
          (`/Game/Ludens_level/Blueprints/Widgets/quote1vr_7.Appear phrase` (`|GetArrayItem` _outactors_2)))))))

(event `/Game/VirtualRealityBP/Blueprints/PickupActorInterface2.Pickup`
  (params (MotionController :type "SceneComponent Object Reference") (HandMesh :type "SceneComponent Object Reference"))
  (`SceneComponent.K2_AttachToComponent` (`self.StaticMeshComponent`) HandMesh "None" "KeepWorld" "KeepWorld" "KeepWorld" false)
  (`/Engine/EditorBlueprintResources/StandardMacros.DoOnce` false
    (:`Completed`
      (bind _outactors (`GameplayStatics.GetAllActorsOfClass` "/Script/Engine.TargetPoint"))
      (bind _returnvalue (`self.K2_GetActorLocation` (`|GetArrayItem` _outactors 5)))
      (`|SpawnActorFromClass` "/Game/Ludens_level/Blueprints/Painting/BP_Whiteboard.BP_Whiteboard_C" (`KismetMathLibrary.MakeTransform` _returnvalue) "Undefined" "OverrideRootScale" null null)
      (`|SpawnActorFromClass` "/Game/Ludens_level/Blueprints/Button/Ereaser.Ereaser_C" (`KismetMathLibrary.MakeTransform` (`KismetMathLibrary.MakeVector` (- (.x _returnvalue) 50.0) (+ (.y _returnvalue) 20.0) (.z _returnvalue)) (struct) (0.3 0.3 0.3)) "Undefined" "OverrideRootScale" null null))))

(event `/Game/VirtualRealityBP/Blueprints/PickupActorInterface2.Drop`
  (params (MotionController :type "SceneComponent Object Reference") (HandMesh :type "SceneComponent Object Reference"))
  (`self.K2_DetachFromActor` "KeepWorld" "KeepWorld" "KeepWorld"))

(event `self.StaticMeshComponent.OnComponentEndOverlap`
  (params (OverlappedComponent :type "PrimitiveComponent Object Reference") (OtherActor :type "Actor Object Reference") (OtherComp :type "PrimitiveComponent Object Reference") (OtherBodyIndex :type Integer))
  (if (== OtherActor (`self.Other Actor`))
    (set `self.ispainting` false)
    (set `self.Other Actor` null)))

(fn `Detect Hit Canvas Actor`)

(fn `HapticsEffect`
  (params (Actor :type "Object Object Reference"))
  (bind _outactors (`GameplayStatics.GetAllActorsOfClass` "/Game/VirtualRealityBP/Blueprints/MotionControllerPawn.MotionControllerPawn_C"))
  (bind _output (`|GetArrayItem` _outactors))
  (bind _leftcontroller (`/Game/VirtualRealityBP/Blueprints/MotionControllerPawn.LeftController` _output))
  (if (== Actor _leftcontroller)
    (`/Game/VirtualRealityBP/Blueprints/BP_MotionController1.RumbleController` _leftcontroller 1.0)
    (else
      (`/Game/VirtualRealityBP/Blueprints/BP_MotionController1.RumbleController` (`/Game/VirtualRealityBP/Blueprints/MotionControllerPawn.RightController` _output) 1.0))))

(fn `UserConstructionScript`)