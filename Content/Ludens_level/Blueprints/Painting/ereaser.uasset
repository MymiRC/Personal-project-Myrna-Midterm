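; VR whiteboard eraser actor that attaches to a motion controller's hand mesh on Pickup and detaches on Drop.
; An overlap enables painting, during which Tick runs a short forward line trace with debug drawing.
; Hits on a BP_Whiteboard pass their collision UV to DrawOnWhiteboard.
; HapticsEffect then rumbles the left or right controller, chosen by comparing the stored overlapping actor to the pawn's left controller.
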(event `self.ReceiveActorBeginOverlap`
  (params (OtherActor :type "Actor Object Reference"))
  (if (== (`self.Other Actor`) null)
    (set `self.Other Actor` OtherActor)
    (set `self.ispainting` true)))

(event `self.StaticMeshComponent.OnComponentEndOverlap`
  (params (OverlappedComponent :type "PrimitiveComponent Object Reference") (OtherActor :type "Actor Object Reference") (OtherComp :type "PrimitiveComponent Object Reference") (OtherBodyIndex :type Integer))
  (if (== OtherActor (`self.Other Actor`))
    (set `self.ispainting` false)
    (set `self.Other Actor` null)))

(event `self.ReceiveTick`
  (params (DeltaSeconds :type "Float (single-precision)"))
  (bind _arrowforward (`self.ArrowForward`))
  (bind _returnvalue (`SceneComponent.K2_GetComponentLocation` _arrowforward))
  (if (`self.ispainting`)
    (bind (_outhit _returnvalue_2) (`KismetSystemLibrary.LineTraceSingle` :`Start` _returnvalue :`End` (+ _returnvalue (* (`KismetMathLibrary.GetForwardVector` (`SceneComponent.K2_GetComponentRotation` _arrowforward)) 15.0)) :`TraceChannel` "TraceTypeQuery1" :`bTraceComplex` true :`DrawDebugType` "ForDuration"))
    (if _returnvalue_2
      (`KismetSystemLibrary.PrintString` "Hello" true true (struct :`R` 0.453834 :`G` 0.02313 :`B` 1.0 :`A` 1.0))
      (bind _asbp_whiteboard (cast `/Game/Ludens_level/Blueprints/Painting/BP_Whiteboard` (`.HitActor` (`GameplayStatics.BreakHitResult` _outhit))))
      (`/Game/Ludens_level/Blueprints/Painting/BP_Whiteboard.DrawOnWhiteboard` _asbp_whiteboard (`GameplayStatics.FindCollisionUV` _outhit))
      (`self.HapticsEffect` (`self.Other Actor`)))))

(event `/Game/VirtualRealityBP/Blueprints/PickupActorInterface2.Pickup`
  (params (MotionController :type "SceneComponent Object Reference") (HandMesh :type "SceneComponent Object Reference"))
  (`SceneComponent.K2_AttachToComponent` (`self.StaticMeshComponent`) HandMesh "None" "KeepWorld" "KeepWorld" "KeepWorld" false))

(event `/Game/VirtualRealityBP/Blueprints/PickupActorInterface2.Drop`
  (params (MotionController :type "SceneComponent Object Reference") (HandMesh :type "SceneComponent Object Reference"))
  (`self.K2_DetachFromActor` "KeepWorld" "KeepWorld" "KeepWorld"))

(fn `Detect Hit Canvas Actor`)

(fn `HapticsEffect`
  (params (Actor :type "Object Object Reference"))
  (bind _outactors (`GameplayStatics.GetAllActorsOfClass` "/Game/VirtualRealityBP/Blueprints/MotionControllerPawn.MotionControllerPawn_C"))
  (bind _output (`|GetArrayItem` _outactors))
  (bind _leftcontroller (`/Game/VirtualRealityBP/Blueprints/MotionControllerPawn.LeftController` _output))
  (if (== Actor _leftcontroller)
    (`/Game/VirtualRealityBP/Blueprints/BP_MotionController1.RumbleController` _leftcontroller 1.0)
    (else
      (`/Game/VirtualRealityBP/Blueprints/BP_MotionController1.RumbleController` (`/Game/VirtualRealityBP/Blueprints/MotionControllerPawn.RightController` _output) 1.0))))

(fn `UserConstructionScript`)